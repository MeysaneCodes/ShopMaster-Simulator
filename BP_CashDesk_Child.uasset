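; Cash desk child Blueprint that fills the desk's computer screen with test item entries when play begins.
; After the parent BeginPlay, it casts the ScreenComputer widget component's user widget to BP_Computer and calls AddIteam in a loop with the same hardcoded name, amount and price.
; A failed cast only prints a debug string.
; Overlap and Tick are disabled stubs, and the construction script only calls the parent.
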(event EventBeginPlay
  (|CallParentFunction)
  (bind _asbp_computer (Utilities|Casting|CastToBP_Computer (UserInterface|GetUserWidgetObject (Variables|Default|GetScreenComputer)))
    (:then
      (for _index (range 0 20)
        (Default|AddIteam _asbp_computer "DB REGIO" 10 299.99)))
    (:CastFailed
      (Development|PrintString "boom"))))

(event Collision|EventActorBeginOverlap
  (params (OtherActor :type Actor%20Object%20Reference))
  (|CallParentFunction OtherActor) ; This node is disabled and will not be called.\nDrag off pins to build functionality.
)

(event EventTick
  (params (DeltaSeconds :type Float%20%28single-precision%29))
  (|CallParentFunction DeltaSeconds) ; This node is disabled and will not be called.\nDrag off pins to build functionality.
)

(fn ConstructionScript
  (|CallParentFunction))