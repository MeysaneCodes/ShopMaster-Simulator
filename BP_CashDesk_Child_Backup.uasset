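; Cash desk actor, a child Blueprint, that registers scanned products on its in-world computer screen.
; When a BP_ItemProduct overlaps ScannerDetector, its name, amount and price are read from ProductDetails and added to the BP_Computer widget in ScreenComputer.
; An IsScanned flag on each product prevents repeat entries.
; BeginPlay only checks the widget cast; test-fill and cursor input logic are left disconnected.
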(event OnComponentBeginOverlap(Box)
  (params (OverlappedComponent :type Primitive%20Component%20Object%20Reference) (OtherActor :type Actor%20Object%20Reference) (OtherComp :type Primitive%20Component%20Object%20Reference) (OtherBodyIndex :type Integer) (bFromSweep :type Boolean) (SweepResult :type Hit%20Result%20Structure%20%28by%20ref%29)))

(event OnComponentBeginOverlap(ScannerDetector)
  (params (OverlappedComponent :type Primitive%20Component%20Object%20Reference) (OtherActor :type Actor%20Object%20Reference) (OtherComp :type Primitive%20Component%20Object%20Reference) (OtherBodyIndex :type Integer) (bFromSweep :type Boolean) (SweepResult :type Hit%20Result%20Structure%20%28by%20ref%29))
  ;[1 1 1] Scanned Items
  (bind _asbp_item_product (Utilities|Casting|CastToBP_ItemProduct OtherActor))
  (if (not (Variables|/Script/Learning.Product|GetbIsScanned _asbp_item_product))
    (bind _asbp_computer (Utilities|Casting|CastToBP_Computer (UserInterface|GetUserWidgetObject (Variables|Default|GetScreenComputer))))
    (Default|AddIteam _asbp_computer (Utilities|Text|ToText(String) (.Value (Utilities|Map|Find (Variables|/Script/Learning.Product|GetProductDetails _asbp_item_product) "Name"))) (Math|Conversions|ToInteger(Byte) (.Value (Utilities|Map|Find (Variables|/Script/Learning.Product|GetProductDetails _asbp_item_product) "Amount"))) (Math|Conversions|ToFloat(Integer) (.Value (Utilities|Map|Find (Variables|/Script/Learning.Product|GetProductDetails _asbp_item_product) "Price"))))
    (Variables|/Script/Learning.Product|SetbIsScanned _asbp_item_product true)))

(event OnComponentBeginOverlap(OverlappingBox)
  (params (OverlappedComponent :type Primitive%20Component%20Object%20Reference) (OtherActor :type Actor%20Object%20Reference) (OtherComp :type Primitive%20Component%20Object%20Reference) (OtherBodyIndex :type Integer) (bFromSweep :type Boolean) (SweepResult :type Hit%20Result%20Structure%20%28by%20ref%29)))

(event EventBeginPlay
  (|CallParentFunction)
  (bind _asbp_computer (Utilities|Casting|CastToBP_Computer (UserInterface|GetUserWidgetObject (Variables|Default|GetScreenComputer)))
    (:CastFailed
      (Development|PrintString "boom"))))

(event Collision|EventActorBeginOverlap
  (params (OtherActor :type Actor%20Object%20Reference))
  (|CallParentFunction OtherActor) ; This node is disabled and will not be called.\nDrag off pins to build functionality.
)

(event EventTick
  (params (DeltaSeconds :type Float%20%28single-precision%29))
  (|CallParentFunction DeltaSeconds) ; This node is disabled and will not be called.\nDrag off pins to build functionality.
)

(fn ConstructionScript
  (|CallParentFunction))